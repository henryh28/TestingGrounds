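; NPC_AI_BP is an AI controller for patrolling NPCs with perception.
; On BeginPlay it sets up the PatrolData blackboard and runs the Patrol behavior tree.
; FindPatrolRoute writes the controlled ThirdPersonCharacter's first patrol point to the Waypoint key of a supplied blackboard; nothing in this file calls it.
; Perception updates only print the pawn, sense class and perceived actor for debugging.
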(event OnTargetPerceptionUpdated(AIPerception)
  (params (Actor :type Actor%20Object%20Reference) (Stimulus :type AI%20Stimulus%20Structure))
  (bind _returnvalue (Class|AIPerceptionSystem|GetSenseClassforStimulus Stimulus))
  (Development|PrintString (Utilities|String|Append (Utilities|GetObjectName (Pawn|GetControlledPawn)) " " (Utilities|GetClassDisplayName _returnvalue) " " (Utilities|GetObjectName Actor))))

(event EventBeginPlay
  (Class|AIController|UseBlackboard "/Game/Blueprints/PatrolData.PatrolData")
  (AI|RunBehaviorTree "/Game/Blueprints/Patrol.Patrol"))

(fn ConstructionScript)

(fn FindPatrolRoute
  (params (Blackboard :type Blackboard%20Component%20Object%20Reference))
  (bind _asthird_person_character (Utilities|Casting|CastToThirdPersonCharacter (Pawn|GetControlledPawn)))
  (AI|Components|Blackboard|SetValueasObject Blackboard (Utilities|Name|MakeLiteralName "Waypoint") (Utilities|Array|Get(acopy) (Variables|/Game/ThirdPersonCPP/Blueprints/ThirdPersonCharacter.ThirdPersonCharacter_C|GetPatrol%20Points _asthird_person_character))))