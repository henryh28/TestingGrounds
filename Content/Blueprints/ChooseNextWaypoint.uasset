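; ChooseNextWaypoint is a Behavior Tree task that sets the patrol waypoint for an AI-controlled pawn.
; It casts the pawn to ThirdPersonCharacter and reads that character's PatrolPoints array.
; It writes the point at the Blackboard's Index to the Waypoint key and finishes successfully, leaving the index itself unchanged.
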(event EventReceiveExecuteAI
  (params (OwnerController :type AI%20Controller%20Object%20Reference) (ControlledPawn :type Pawn%20Object%20Reference))
  (CallFunction|GetPatrolPoints ControlledPawn)
  (Class|BTFunctionLibrary|SetBlackboardValueasObject (Variables|Default|GetWaypoint) (Utilities|Array|Get(acopy) (Variables|Default|GetPatrol%20Points) (Class|BTFunctionLibrary|GetBlackboardValueasInt (Variables|Default|GetIndex))))
  (AI|BehaviorTree|FinishExecute true))

(fn GetPatrolPoints
  (params (Object :type Object%20Object%20Reference))
  (bind _asthird_person_character (Utilities|Casting|CastToThirdPersonCharacter Object))
  (Variables|Default|SetPatrol%20Points (Variables|/Game/ThirdPersonCPP/Blueprints/ThirdPersonCharacter.ThirdPersonCharacter_C|GetPatrol%20Points _asthird_person_character)))